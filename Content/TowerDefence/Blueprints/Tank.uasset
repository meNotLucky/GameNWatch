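; Tank Blueprint for the tower defence game, whose type sets both its hit points and its appearance.
; Instantiate clamps the type into a small health range, and UpdateMesh looks up the static mesh for that health in the Meshes map.
; Each TakeDamage call removes one health and swaps the mesh; at the last point it flags IsDead and hides the mesh without destroying the tank.
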(event EventTick
  (params (DeltaSeconds :type Float%20%28single-precision%29)))

(fn ConstructionScript)

(fn Instantiate
  (params (TankType :type Integer))
  (Variables|Default|Sethealth (Math|Integer|Clamp(Integer) TankType 1 3))
  (CallFunction|UpdateMesh))

(fn UpdateMesh
  (Components|StaticMesh|SetStaticMesh (Variables|Default|GetStaticMesh) (.Value (Utilities|Map|Find (Variables|Default|Getmeshes) (Variables|Default|Gethealth)))))

(fn TakeDamage
  (if (> (Variables|Default|Gethealth) 1)
    (bind _result (Math|Integer|DecrementInt (Variables|Default|Gethealth))
      (:%20%20
        (Variables|Default|Sethealth _result)
        (CallFunction|UpdateMesh)))
    (else
      (Variables|Default|SetisDead true)
      (Rendering|SetVisibility (Variables|Default|GetStaticMesh) false false))))