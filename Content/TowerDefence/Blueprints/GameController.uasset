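; Tower defence controller that lets the player cycle through turret slots and turret types with the keyboard.
; A/D step the slot index and W/S the type index, using helper functions that wrap around the array ends.
; Every Tick it resolves both selections and loops over each array, showing only the selected slot's highlight and the selected type's mesh.
; No turret placement is implemented here.
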(event Custom|Update%20Slot%20Selection
  (Variables|Default|SetselectedTurretSlot (Utilities|Array|Get(acopy) (Variables|Default|GetturretSlots) (Variables|Default|GetselectedSlotIndex)))
  (for _array_element (Variables|Default|GetturretSlots)
    (if (== _array_element (Variables|Default|GetselectedTurretSlot))
      (Rendering|SetVisibility (Variables|/Game/TowerDefence/Blueprints/TurretSlot.TurretSlot_C|GetHighlight _array_element) true true)
      (else
        (Rendering|SetVisibility (Variables|/Game/TowerDefence/Blueprints/TurretSlot.TurretSlot_C|GetHighlight _array_element) false true)))))

(event Custom|Update%20Type%20Selection
  (Variables|Default|SetselectedTurretType (Utilities|Array|Get(acopy) (Variables|Default|GetturretTypes) (Variables|Default|GetselectedTypeIndex)))
  (for _array_element (Variables|Default|GetturretTypes)
    (if (== _array_element (Variables|Default|GetselectedTurretType))
      (Rendering|SetVisibility (Variables|/Game/TowerDefence/Blueprints/TurretType.TurretType_C|GetStaticMesh _array_element) true true)
      (else
        (Rendering|SetVisibility (Variables|/Game/TowerDefence/Blueprints/TurretType.TurretType_C|GetStaticMesh _array_element) false true)))))

(event EventTick
  (params (DeltaSeconds :type Float%20%28single-precision%29))
  (CallFunction|UpdateSlotSelection)
  (CallFunction|UpdateTypeSelection))

(event Input|KeyboardEvents|D
  (params (Key :type Key%20Structure :default "None"))
  (:Pressed
    (bind _newindex (CallFunction|SelectNext (Variables|Default|GetselectedSlotIndex) (Utilities|Array|Length (Variables|Default|GetturretSlots))))
    (Variables|Default|SetselectedSlotIndex _newindex)))

(event Input|KeyboardEvents|A
  (params (Key :type Key%20Structure :default "None"))
  (:Pressed
    (bind _newindex (CallFunction|SelectPrevious (Variables|Default|GetselectedSlotIndex) (Utilities|Array|Length (Variables|Default|GetturretSlots))))
    (Variables|Default|SetselectedSlotIndex _newindex)))

(event Input|KeyboardEvents|W
  (params (Key :type Key%20Structure :default "None"))
  (:Pressed
    (bind _newindex (CallFunction|SelectPrevious (Variables|Default|GetselectedTypeIndex) (Utilities|Array|Length (Variables|Default|GetturretTypes))))
    (Variables|Default|SetselectedTypeIndex _newindex)))

(event Input|KeyboardEvents|S
  (params (Key :type Key%20Structure :default "None"))
  (:Pressed
    (bind _newindex (CallFunction|SelectNext (Variables|Default|GetselectedTypeIndex) (Utilities|Array|Length (Variables|Default|GetturretTypes))))
    (Variables|Default|SetselectedTypeIndex _newindex)))

(fn ConstructionScript)

(fn SelectNext
  (params (currentIndex :type Integer) (lenght :type Integer))
  (bind _result (Math|Integer|IncrementInt currentIndex)
    (:%20%20
      (if (< _result lenght)
        (return _result)
        (else
          (return 0))))))

(fn SelectPrevious
  (params (currentIndex :type Integer) (lenght :type Integer))
  (bind _result (Math|Integer|DecrementInt currentIndex)
    (:%20%20
      (if (> _result -1)
        (return _result)
        (else
          (return (- lenght 1)))))))

(fn NewFunction0
  (params (NewParam :type Array%20of%20Actor%20Object%20References)))