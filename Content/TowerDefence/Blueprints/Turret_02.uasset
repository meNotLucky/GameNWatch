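; Turret_02 is a tower defence turret variant that kills every Tank inside its two colliders when it fires.
; A Tank entering Collider1 starts the firing sequence if the turret is activated and its cooldown timer is zero.
; The BeginFireingSequence override runs the parent logic, then calls Fire, which waits briefly and sets IsDead on all Tanks overlapping Collider1 and Collider.
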(event OnComponentBeginOverlap(Collider1)
  (params (OverlappedComponent :type Primitive%20Component%20Object%20Reference) (OtherActor :type Actor%20Object%20Reference) (OtherComp :type Primitive%20Component%20Object%20Reference) (OtherBodyIndex :type Integer) (bFromSweep :type Boolean) (SweepResult :type Hit%20Result%20Structure%20%28by%20ref%29))
  (if (Math|Boolean|ANDBoolean (Variables|Default|Getactivated) (== (Utilities|GetClass OtherActor) "/Game/TowerDefence/Blueprints/Tank.Tank_C") (== (Variables|Default|GetcooldownTimer) 0.0))
    (CallFunction|BeginFireingSequence)))

(event Custom|Fire
  (Utilities|FlowControl|Delay 0.1)
  (for _array_element (Collision|GetOverlappingActors (Variables|Default|GetCollider1) "/Game/TowerDefence/Blueprints/Tank.Tank_C" :!class /Script/Engine.PrimitiveComponent)
    (bind _astank (Utilities|Casting|CastToTank _array_element))
    (Variables|/Game/TowerDefence/Blueprints/Tank.Tank_C|SetisDead _astank true))
  (for _array_element_2 (Collision|GetOverlappingActors (Variables|Default|GetCollider) "/Game/TowerDefence/Blueprints/Tank.Tank_C" :!class /Script/Engine.PrimitiveComponent)
    (bind _astank_2 (Utilities|Casting|CastToTank _array_element_2))
    (Variables|/Game/TowerDefence/Blueprints/Tank.Tank_C|SetisDead _astank_2 true)))

(event EventBeginPlay
  (|CallParentFunction) ; This node is disabled and will not be called.\nDrag off pins to build functionality.
)

(event Collision|EventActorBeginOverlap
  (params (OtherActor :type Actor%20Object%20Reference))
  (|CallParentFunction OtherActor) ; This node is disabled and will not be called.\nDrag off pins to build functionality.
)

(event EventTick
  (params (DeltaSeconds :type Float%20%28single-precision%29))
  (|CallParentFunction DeltaSeconds) ; This node is disabled and will not be called.\nDrag off pins to build functionality.
)

(fn ConstructionScript
  (|CallParentFunction))

(fn BeginFireingSequence
  (|CallParentFunction)
  (CallFunction|Fire))