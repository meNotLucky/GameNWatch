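; Tower defence turret Blueprint that reacts to Tank actors entering its collider and shows its barrel only while activated.
; An overlap begin starts the firing sequence if the turret is active and off cooldown, setting the firing flag and cooldown timer.
; Tick counts the timer down and clears the flag at zero.
; The sequence contains no projectile or damage logic.
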(event OnComponentBeginOverlap(Collider)
  (params (OverlappedComponent :type Primitive%20Component%20Object%20Reference) (OtherActor :type Actor%20Object%20Reference) (OtherComp :type Primitive%20Component%20Object%20Reference) (OtherBodyIndex :type Integer) (bFromSweep :type Boolean) (SweepResult :type Hit%20Result%20Structure%20%28by%20ref%29))
  (if (Math|Boolean|ANDBoolean (Variables|Default|Getactivated) (== (Utilities|GetClass OtherActor) "/Game/TowerDefence/Blueprints/Tank.Tank_C") (== (Variables|Default|GetcooldownTimer) 0.0))
    (CallFunction|BeginFireingSequence)))

(event Custom|Update%20Cooldown%20Timer
  (bind _output_get (Variables|Default|SetcooldownTimer (- (Variables|Default|GetcooldownTimer) (stale EventTick DeltaSeconds))))
  (if (<= _output_get 0.0)
    (Variables|Default|Setfiering false)
    (Variables|Default|SetcooldownTimer 0.0)))

(event EventTick
  (params (DeltaSeconds :type Float%20%28single-precision%29))
  (bind _barrel (Variables|Default|GetBarrel))
  (if (Variables|Default|Getactivated)
    (Rendering|SetVisibility _barrel true true)
    (if (Variables|Default|Getfiering)
      (CallFunction|UpdateCooldownTimer))
    (else
      (Rendering|SetVisibility _barrel false true))))

(fn ConstructionScript)

(fn BeginFireingSequence
  (Variables|Default|Setfiering true)
  (Variables|Default|SetcooldownTimer (Variables|Default|Getcooldown)))