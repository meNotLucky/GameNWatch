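; Turret_03 is a tower defence turret that kills every tank inside its collider each time it fires, acting as an area attack.
; It overrides BeginFireingSequence, running the parent's sequence and then triggering the DelayedFire event.
; After a short delay, DelayedFire gathers the Tank actors overlapping the collider and sets IsDead on each directly, with no damage calculation.
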(event Custom|DelayedFire
  (Utilities|FlowControl|Delay 0.2)
  (for _array_element (Collision|GetOverlappingActors (Variables|Default|GetCollider) "/Game/TowerDefence/Blueprints/Tank.Tank_C" :!class /Script/Engine.PrimitiveComponent)
    (bind _astank (Utilities|Casting|CastToTank _array_element))
    (Variables|/Game/TowerDefence/Blueprints/Tank.Tank_C|SetisDead _astank true)))

(event EventBeginPlay
  (|CallParentFunction) ; This node is disabled and will not be called.\nDrag off pins to build functionality.
)

(event Collision|EventActorBeginOverlap
  (params (OtherActor :type Actor%20Object%20Reference))
  (|CallParentFunction OtherActor) ; This node is disabled and will not be called.\nDrag off pins to build functionality.
)

(event EventTick
  (params (DeltaSeconds :type Float%20%28single-precision%29))
  (|CallParentFunction DeltaSeconds) ; This node is disabled and will not be called.\nDrag off pins to build functionality.
)

(fn ConstructionScript
  (|CallParentFunction))

(fn BeginFireingSequence
  (|CallParentFunction)
  (CallFunction|DelayedFire))